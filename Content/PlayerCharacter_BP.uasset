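; Player character Blueprint for a sword-wielding character, handling movement, attacking and ragdolling.
; Axis inputs move along world X and Y, turning the mesh to face velocity with a yaw offset.
; Attack presses drive Assignment_AnimBP, gated by animation length; StopAttacking uses a short timer, cancelled by another press, before ending the attack.
; Ragdoll enables mesh physics, disables movement and drops the sword, while IsAttacking exposes the AnimBP's state.
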(event Custom|Stop%20Anims
  ;[1 1 1] Delay the ending of animation
  (bind _asassignment_anim_bp (Utilities|Casting|CastToAssignment_AnimBP (Components|SkeletalMesh|GetAnimInstance (Variables|Character|GetMesh))))
  (Default|StopAttacking _asassignment_anim_bp)
  (Variables|Default|SetLastAttackTime 0.0))

(event EventBeginPlay)

(event Collision|EventActorBeginOverlap
  (params (OtherActor :type Actor%20Object%20Reference)))

(event EventTick
  (params (DeltaSeconds :type Float%20%28single-precision%29)))

(event EventRagdoll
  (bind _mesh (Variables|Character|GetMesh))
  (bind _swordmesh (Variables|Default|GetSwordMesh))
  ;[1 1 1] RAGDOLL
  (Utilities|FlowControl|Sequence
    (:then_0
      ;;[1 1 1] Ragdoll the player Mesh
      (Collision|SetCollisionProfileName _mesh "Ragdoll" true :!class /Script/Engine.PrimitiveComponent)
      (Physics|SetSimulatePhysics _mesh true))
    (:then_1
      ;;[1 1 1] Disallow Player Movement
      (Pawn|Components|CharacterMovement|DisableMovement (Variables|Character|GetCharacterMovement)))
    (:then_2
      ;;[1 1 1] Drop the sword
      (Transformation|DetachFromComponent _swordmesh "KeepRelative" "KeepRelative" "KeepRelative" true)
      (Collision|SetCollisionProfileName _swordmesh "BlockAll" true :!class /Script/Engine.PrimitiveComponent)
      (Physics|SetSimulatePhysics _swordmesh true))))

(event EventStopAttacking
  (bind _returnvalue (Utilities|Time|SetTimerbyEvent (delegate Custom|Stop%20Anims) 0.1))
  (Variables|Default|SetStopAnimsTimerHandle _returnvalue))

(event Input|ActionEvents|InputActionAttack
  (params (Key :type Key%20Structure :default "None"))
  ;[1 1 1] Not the best way of Implementing this, but you're writting C++ code, so maybe focus on that ;)
  (:Pressed
    (Utilities|Time|ClearandInvalidateTimerbyHandle (Variables|Default|GetStopAnimsTimerHandle))
    (if (> (- (Utilities|Time|GetTimeSeconds) (Variables|Default|GetLastAttackTime)) (Variables|Default|GetAttackAnimLength))
      (bind _asassignment_anim_bp (Utilities|Casting|CastToAssignment_AnimBP (Components|SkeletalMesh|GetAnimInstance (Variables|Character|GetMesh))))
      (Default|StartAttacking _asassignment_anim_bp)
      (Variables|Default|SetLastAttackTime (Utilities|Time|GetTimeSeconds)))))

(event Input|AxisEvents|InputAxisMoveForward
  (params (AxisValue :type Float%20%28single-precision%29))
  (bind _charactermovement (Variables|Character|GetCharacterMovement))
  (bind _velocity (Variables|/Script/Engine.MovementComponent|GetVelocity _charactermovement))
  (bind _returnvalue (Math|Rotator|MakeRotationfromAxes _velocity "0, 0, 0" "0, 0, 0"))
  (bind (_roll _pitch _yaw) (Math|Rotator|BreakRotator _returnvalue))
  ;[1 1 1] Movement code
  (if (!= AxisValue 0.0)
    (Class|PawnMovementComponent|AddInputVector (Variables|Character|GetCharacterMovement) (Math|Vector|MakeVector AxisValue 0.0 0.0) false)
    (Transformation|SetWorldRotation (Variables|Character|GetMesh) (Math|Rotator|MakeRotator _roll _pitch (+ _yaw -9e+01)) false false)))

(event Input|AxisEvents|InputAxisMoveRight
  (params (AxisValue :type Float%20%28single-precision%29))
  (bind _charactermovement (Variables|Character|GetCharacterMovement))
  (bind _velocity (Variables|/Script/Engine.MovementComponent|GetVelocity _charactermovement))
  (bind _returnvalue (Math|Rotator|MakeRotationfromAxes _velocity "0, 0, 0" "0, 0, 0"))
  (bind (_roll _pitch _yaw) (Math|Rotator|BreakRotator _returnvalue))
  ;[1 1 1] Movement code
  (if (!= AxisValue 0.0)
    (Class|PawnMovementComponent|AddInputVector (Variables|Character|GetCharacterMovement) (Math|Vector|MakeVector 0.0 AxisValue 0.0) false)
    (Transformation|SetWorldRotation (Variables|Character|GetMesh) (Math|Rotator|MakeRotator _roll _pitch (+ _yaw -9e+01)) false false)))

(fn ConstructionScript)

(fn IsAttacking
  (bind _asassignment_anim_bp (Utilities|Casting|CastToAssignment_AnimBP (Components|SkeletalMesh|GetAnimInstance (Variables|Character|GetMesh))))
  (return (Variables|/Game/Animations/Assignment_AnimBP.Assignment_AnimBP_C|GetIsAttacking _asassignment_anim_bp)))