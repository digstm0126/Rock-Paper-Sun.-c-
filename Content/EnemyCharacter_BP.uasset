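; Enemy character Blueprint that relays attack animation state to its Assignment_AnimBP and handles ragdolling.
; StartAttacking cancels any pending stop and only retriggers the anim once the attack anim length has elapsed since the last attack.
; StopAttacking ends the anim after a short timer delay and resets the attack time, while IsAttacking reads the anim blueprint's flag.
; Ragdoll enables mesh physics, disables movement and removes capsule collision.
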(event Custom|Stop%20Anims
  ;[1 1 1] Delay the ending of animation
  (bind _asassignment_anim_bp (Utilities|Casting|CastToAssignment_AnimBP (Components|SkeletalMesh|GetAnimInstance (Variables|Character|GetMesh))))
  (Default|StopAttacking _asassignment_anim_bp)
  (Variables|Default|SetLastAttackTime 0.0))

(event EventBeginPlay)

(event Collision|EventActorBeginOverlap
  (params (OtherActor :type Actor%20Object%20Reference)))

(event EventTick
  (params (DeltaSeconds :type Float%20%28single-precision%29)))

(event EventStartAttacking
  ;[1 1 1] Causes the anim blueprint to record an attack time, triggering a singular anim
  (Utilities|Time|ClearandInvalidateTimerbyHandle (Variables|Default|GetStopAnimsTimerHandle))
  (if (> (- (Utilities|Time|GetTimeSeconds) (Variables|Default|GetLastAttackTime)) (Variables|Default|GetAttackAnimLength))
    (bind _asassignment_anim_bp (Utilities|Casting|CastToAssignment_AnimBP (Components|SkeletalMesh|GetAnimInstance (Variables|Character|GetMesh))))
    (Default|StartAttacking _asassignment_anim_bp)
    (Variables|Default|SetLastAttackTime (Utilities|Time|GetTimeSeconds))))

(event EventStopAttacking
  (bind _returnvalue (Utilities|Time|SetTimerbyEvent (delegate Custom|Stop%20Anims) 0.1))
  (Variables|Default|SetStopAnimsTimerHandle _returnvalue))

(event EventRagdoll
  (bind _mesh (Variables|Character|GetMesh))
  ;[1 1 1] RAGDOLL
  (Utilities|FlowControl|Sequence
    (:then_0
      ;;[1 1 1] Ragdoll the Enemy Mesh
      (Collision|SetCollisionProfileName _mesh "RagDoll" true :!class /Script/Engine.PrimitiveComponent)
      (Physics|SetSimulatePhysics _mesh true))
    (:then_1
      ;;[1 1 1] Disallow Player Movement
      (Pawn|Components|CharacterMovement|DisableMovement (Variables|Character|GetCharacterMovement)))
    (:then_2
      (Collision|SetCollisionProfileName (Variables|Default|GetCapsuleComponent) "NoCollision" true :!class /Script/Engine.PrimitiveComponent))))

(fn ConstructionScript)

(fn IsAttacking
  (bind _asassignment_anim_bp (Utilities|Casting|CastToAssignment_AnimBP (Components|SkeletalMesh|GetAnimInstance (Variables|Character|GetMesh))))
  (return (Variables|/Game/Animations/Assignment_AnimBP.Assignment_AnimBP_C|GetIsAttacking _asassignment_anim_bp)))